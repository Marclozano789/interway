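; BP_Target is a drone-game target actor whose static mesh travels along its own spline path.
; Each Tick it advances the distance by Speed times delta time and sets the mesh's world location and rotation from the spline.
; The distance resets to zero at the spline's end, so movement loops.
; The mesh's hit event is empty, and a DestroyActor call is left unconnected, so hits have no effect here.
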(event `self.ReceiveTick`
  (params (DeltaSeconds :type "Float (single-precision)"))
  (bind _output_get (set `self.DistanceAlongSpline` (+ (* (`self.Speed`) (`GameplayStatics.GetWorldDeltaSeconds`)) (`self.DistanceAlongSpline`))))
  (`SceneComponent.K2_SetWorldLocationAndRotation` (`self.StaticMesh`) (`SplineComponent.GetLocationAtDistanceAlongSpline` (`self.Spline`) _output_get "World") (`SplineComponent.GetRotationAtDistanceAlongSpline` (`self.Spline`) _output_get "World") false false)
  (if (>= (`self.DistanceAlongSpline`) (`SplineComponent.GetSplineLength` (`self.Spline`)))
    (set `self.DistanceAlongSpline` 0.0)))

(event `self.StaticMesh.OnComponentHit`
  (params (HitComponent :type "PrimitiveComponent Object Reference") (OtherActor :type "Actor Object Reference") (OtherComp :type "PrimitiveComponent Object Reference") (NormalImpulse :type "Vector Structure") (Hit :type "HitResult Structure (by ref)")))

(fn `UserConstructionScript`)