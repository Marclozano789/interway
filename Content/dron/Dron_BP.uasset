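; Player-controlled drone that flies by physics and shoots projectiles.
; Input axes drive mass-independent forces and torques on the static mesh along its own axes, with thrust along the right vector and rotation about all three axes.
; Ascend applies a single upward force per press and prints a debug string.
; Shoot spawns BP_Projectile at MuzzleLocation, then sets its movement's initial speed after spawning.
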(event `InputAxis|Accelerar`
  (params (AxisValue :type "Float (single-precision)"))
  ;[0 0.5952 0.849 0.5] Accelerar
  (`PrimitiveComponent.AddForce` (`self.StaticMesh`) (* (`SceneComponent.GetRightVector` (`self.StaticMesh`)) (* AxisValue 1800.0)) "None" true))

(event `InputAction|IA_Ascend`
  (params (Key :type "Key Structure"))
  ; Ascender
  (:`Pressed`
    (`PrimitiveComponent.AddForce` (`self.StaticMesh`) (* (`SceneComponent.GetUpVector` (`self.StaticMesh`)) 30000.0) "None" true)
    (`KismetSystemLibrary.PrintString` "Hello")))

(event `InputAxis|derechaizquierda`
  (params (AxisValue :type "Float (single-precision)"))
  ;[0.07089 0.15 0.03196 0.5] Derecha-Izquierda
  (`PrimitiveComponent.AddTorqueInDegrees` (`self.StaticMesh`) (* (`SceneComponent.GetUpVector` (`self.StaticMesh`)) (* AxisValue 50.0)) "None" true))

(event `InputAxis|girar`
  (params (AxisValue :type "Float (single-precision)"))
  ;[0.15 0.02082 0.02333 0.5] Girar
  (`PrimitiveComponent.AddTorqueInDegrees` (`self.StaticMesh`) (* (`SceneComponent.GetRightVector` (`self.StaticMesh`)) (* AxisValue 50.0)) "None" true))

(event `InputAxis|subirbajar`
  (params (AxisValue :type "Float (single-precision)"))
  ;[0.15 0.04367 0.1401 0.5] Subir-bajar
  (`PrimitiveComponent.AddTorqueInDegrees` (`self.StaticMesh`) (* (`SceneComponent.GetForwardVector` (`self.StaticMesh`)) (* AxisValue 50.0)) "None" true))

(event `InputAction|IA_Shoot`
  (params (Key :type "Key Structure"))
  ;[0.8802 0.7842 0.1386 0.5] Disparo
  (:`Pressed`
    (bind _returnvalue (`|SpawnActorFromClass` "/Game/dron/disparos_y_cosas/BP_Projectile.BP_Projectile_C" (`SceneComponent.K2_GetComponentToWorld` (`self.Muzzle_Location`)) "Undefined" "MultiplyWithRoot" null null))
    (set `ProjectileMovementComponent.InitialSpeed` 1000.0 (`/Game/dron/disparos_y_cosas/BP_Projectile.ProjectileMovement` _returnvalue))))

(fn `UserConstructionScript`)